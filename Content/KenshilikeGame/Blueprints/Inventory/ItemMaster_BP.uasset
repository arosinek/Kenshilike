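; ItemMaster_BP is the base actor for world items that units pick up.
; Its construction script stores the actor's own class in ItemData, which BeginPlay passes to the floating name widget.
; Each Tick toggles that label to match the player controller's ShowItemLabels flag.
; When a UnitMasterBP overlaps the sphere and CanBePickedUp is set, it calls TryAddItem with ItemData and destroys itself, without checking the result.
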(event `self.ReceiveBeginPlay`
  ;[1 1 1] Casts
  (bind _asplayer_controller_bp (cast `/Game/KenshilikeGame/Blueprints/Player/PlayerController_BP` (`GameplayStatics.GetPlayerController` 0)))
  (set `self.As Player Controller BP` _asplayer_controller_bp)
  (bind _asitem_floating_name_hud (cast `/Game/KenshilikeGame/Blueprints/Inventory/ItemFloatingName_HUD` (`WidgetComponent.GetUserWidgetObject` (`self.Widget`))))
  (set `/Game/KenshilikeGame/Blueprints/Inventory/ItemFloatingName_HUD.ItemData` (`self.ItemData`) _asitem_floating_name_hud))

(event `self.ReceiveTick`
  (params (DeltaSeconds :type "Float (single-precision)"))
  (bind _widget (`self.Widget`))
  ;[1 1 1] ItemFloatingName Visibility
  (if (`/Game/KenshilikeGame/Blueprints/Player/PlayerController_BP.ShowItemLabels` (`self.As Player Controller BP`))
    (`SceneComponent.SetVisibility` _widget true false)
    (else
      (`SceneComponent.SetVisibility` _widget false false))))

(event `self.Sphere.OnComponentBeginOverlap`
  (params (OverlappedComponent :type "PrimitiveComponent Object Reference") (OtherActor :type "Actor Object Reference") (OtherComp :type "PrimitiveComponent Object Reference") (OtherBodyIndex :type Integer) (bFromSweep :type Boolean) (SweepResult :type "HitResult Structure (by ref)"))
  ;[1 1 1] ItemPickUp
  (bind _asunit_master_bp (cast `/Game/KenshilikeGame/Blueprints/Units/UnitMasterBP` OtherActor))
  (if (`self.CanBePickedUp?`)
    (`KismetSystemLibrary.Delay` 0.0)
    (`/Game/KenshilikeGame/Blueprints/Units/UnitMasterBP.TryAddItem` _asunit_master_bp (`self.ItemData`))
    (set `self.CanBePickedUp?` false)
    (`self.K2_DestroyActor`)))

(fn `UserConstructionScript`
  (setmembers `/Game/KenshilikeGame/Blueprints/Inventory/ItemData_Struct` :`StructRef` (`self.ItemData`) :`ItemClass` (`GameplayStatics.GetObjectClass` self)))