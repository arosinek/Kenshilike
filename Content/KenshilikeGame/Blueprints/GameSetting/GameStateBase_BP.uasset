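; Game state Blueprint that runs the in-game clock and calendar, with 30-day months and 12-month years.
; Tick advances time by game speed through SetGameTime, derives clock and date values, and pushes both to the player controller's timer HUD.
; When the day count is one, it gathers every UnitMasterBP actor for a birthday check.
; UpdateGameSpeed scales the default speed by a multiplier and passes it to CallGameSpeedControl.
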(event `self.ReceiveBeginPlay`
  (`|ExecutionSequence`
    (:`then_0`
      (`self.ReferenceCast`))
    (:`then_1`
      ;[1 1 1] SetInitialTime
      (set `self.GameTime` (+ (`KismetMathLibrary.Conv_IntToDouble` (`self.Hours`)) (/ (`KismetMathLibrary.Conv_IntToDouble` (`self.Minutes`)) 60.0) (/ (`KismetMathLibrary.Conv_IntToDouble` (`self.Hours`)) 3600.0)))
      ;[1 1 1] MakeCalendar
      (set `self.GameDate` (`|MakeArray` (`self.Day`) (`self.Month`) (`self.Year`))))
    (:`then_2`
      ;[1 1 1] DefaultGameSpeed
      (set `self.GameSpeed` (`self.DefaultGameSpeed`)))))

(event `self.ReceiveTick`
  (params (DeltaSeconds :type "Float (single-precision)"))
  (bind (_gametime _daycount) (`/Game/KenshilikeGame/Blueprints/Libraries/FunctionLibrary_BP.SetGameTime` DeltaSeconds (`self.GameSpeed`) (`self.GameTime`)))
  ;[1 1 1] InitializeTime
  (set `self.GameTime` _gametime)
  (set `self.DayCounter` _daycount)
  ;[1 1 1] SetClock&Calendar
  (`self.SetClock`)
  (`self.SetCalendar`)
  ;[1 1 1] BirthDayCheck
  (if (== _daycount 1)
    (bind _unitout (`self.GetAllUnits`))
    (for _array_element _unitout
      (`/Game/KenshilikeGame/Blueprints/Units/UnitMasterBP.BirthDayCheck` _array_element))))

(event `/Game/KenshilikeGame/Blueprints/Libraries/GameTimeInterface_BP.UpdateGameSpeed`
  (params (SpeedMultiplier :type "Float (single-precision)"))
  ;[1 1 1] UpdateGameSpeed
  (bind _output_get (set `self.SpeedMultiplier` SpeedMultiplier))
  (bind _output_get_2 (set `self.GameSpeed` (* _output_get (`self.DefaultGameSpeed`))))
  (`self.GameSpeedControl` _output_get_2))

(fn `GetAllUnits`
  (returns (UnitOut :type "Array of /Game/KenshilikeGame/Blueprints/Units/UnitMasterBP Object Reference"))
  (bind _outactors (`GameplayStatics.GetAllActorsOfClass` "/Game/KenshilikeGame/Blueprints/Units/UnitMasterBP.UnitMasterBP_C"))
  (bind _output_get (set `self.ListOfAllUnits` _outactors))
  (return _output_get))

(fn `GetGameSpeed`
  (returns (GameSpeed :type "Float (double-precision)"))
  (return (`self.GameSpeed`)))

(fn `SetCalendar`
  (bind _output_get (set `self.Day` (+ (`self.Day`) (`self.DayCounter`))))
  (if (> _output_get 30)
    (set `self.Day` 1)
    (bind _result (`/Engine/EditorBlueprintResources/StandardMacros.IncrementInt` (`self.Month`))
      (:`  `
        _)))
  (if (> _result 12)
    (set `self.Month` 1)
    (`/Engine/EditorBlueprintResources/StandardMacros.IncrementInt` (`self.Year`)
      (:`  `
        _)))
  (bind _output_get_2 (set `self.GameDate` (`|MakeArray` (`self.Day`) (`self.Month`) (`self.Year`))))
  (message `/Game/KenshilikeGame/Blueprints/Libraries/GameTimeInterface_BP.SetGameCalendar` (`/Game/KenshilikeGame/Blueprints/Player/PlayerController_BP.GameTimerRef_HUD` (`self.PlayerControllerRef`)) _output_get_2))

(fn `SetClock`
  (bind (_remainder _returnvalue) (`KismetMathLibrary.FMod` (* (`self.GameTime`) 3600.0) 60.0))
  (bind (_remainder_2 _returnvalue_2) (`KismetMathLibrary.FMod` (`KismetMathLibrary.Conv_IntToDouble` _returnvalue) 60.0))
  (set `self.Seconds` (`KismetMathLibrary.FFloor` _remainder))
  (set `self.Minutes` (`KismetMathLibrary.FFloor` _remainder_2))
  (set `self.Hours` (`KismetMathLibrary.FFloor` (`KismetMathLibrary.FMod` (`KismetMathLibrary.Conv_IntToDouble` _returnvalue_2) 24.0)))
  (bind _output_get (set `self.GameDate` (`|MakeArray` (`self.Seconds`) (`self.Minutes`) (`self.Hours`))))
  (message `/Game/KenshilikeGame/Blueprints/Libraries/GameTimeInterface_BP.SetGameClock` (`/Game/KenshilikeGame/Blueprints/Player/PlayerController_BP.GameTimerRef_HUD` (`self.PlayerControllerRef`)) _output_get))

(fn `SetGameCalendar`
  (params (GameDate :type "Array of Integer (by ref)"))
  (returns (Success :type Boolean))
  (return false))

(fn `SetGameClock`
  (params (GameTime :type "Array of Integer (by ref)"))
  (returns (Success :type Boolean))
  (return false))

(fn `UserConstructionScript`)