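; HUD Blueprint that provides RTS-style marquee selection of units and vehicles.
; Input start records the mouse corner and clears the previous selection unless Shift is held; holding moves the opposite corner.
; While dragging, DrawHUD draws the rectangle and gathers actors inside it with GetActorsInSelectionRectangle.
; Release sets selection decals and passes both lists to PlayerController_BP, though SetVehicles sets IsSelected to false on selected vehicles.
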(event `/Game/KenshilikeGame/Blueprints/Libraries/MarqueeSelection_BP.OnInputStart`
  (bind (_locationx _locationy) (`PlayerController.GetMousePosition` (`self.PlayerControllerRef`)))
  ;[1 1 1] OnInputStart
  (if (or (>= (`KismetArrayLibrary.Array_LastIndex` (`self.SelectedUnits`)) 0) (>= (`KismetArrayLibrary.Array_LastIndex` (`self.Selected Vehicles`)) 0))
    (if (`/Game/KenshilikeGame/Blueprints/Player/PlayerController_BP.IsShiftPressed?` (`self.PlayerControllerRef`))
      (bind _output_get (set `self.ClickLocation` (`KismetMathLibrary.MakeVector2D` _locationx _locationy) :!label _label))
      (set `self.HoldingLocation` _output_get)
      (set `self.IsDrawing` true)
      (else
        (`|ExecutionSequence`
          (:`then_0`
            ;;[1 1 1] DeselectUnits
            (`self.ClearSelectedUnits`))
          (:`then_1`
            ;;[1 1 1] DeselectVehicles
            (`self.ClearSelectedVehicles`))
          (:`then_2`
            ;;[1 1 1] SelectedUnits
            (`/Game/KenshilikeGame/Blueprints/Player/PlayerController_BP.Set Selected Units` (`self.PlayerControllerRef`) (`self.SelectedUnits`) (`self.Selected Vehicles`))
            (goto _label)))))
    (else
      (goto _label))))

(event `/Game/KenshilikeGame/Blueprints/Libraries/MarqueeSelection_BP.OnInputRelease`
  (params (HoldTime :type "Float (single-precision)"))
  ;[1 1 1] OnInputRelease
  (set `self.IsDrawing` false)
  (`self.SetUnits`)
  (`self.SetVehicles`)
  (`/Game/KenshilikeGame/Blueprints/Player/PlayerController_BP.Set Selected Units` (`self.PlayerControllerRef`) (`self.SelectedUnits`) (`self.Selected Vehicles`)))

(event `DrawMarquee`
  (bind (_clicklocation_x _clicklocation_y) (`KismetMathLibrary.BreakVector2D` (`self.ClickLocation`)))
  (bind (_holdinglocation_x _holdinglocation_y) (`KismetMathLibrary.BreakVector2D` (`self.HoldingLocation`)))
  (bind _clicklocation (`self.ClickLocation`))
  (bind (_returnvalue_x _returnvalue_y) (`KismetMathLibrary.BreakVector2D` (- (`self.HoldingLocation`) _clicklocation)))
  (bind (_x _y) (`KismetMathLibrary.BreakVector2D` _clicklocation))
  ;[1 1 1] DrawMarquee
  (`self.DrawRect` (struct :`A` 1.0) _clicklocation_x _clicklocation_y)
  (`self.DrawRect` (struct :`A` 1) _holdinglocation_x _holdinglocation_y)
  (`self.DrawRect` (struct :`R` 0.031194 :`G` 0.414618 :`B` 1.0 :`A` 0.567) _x _y _returnvalue_x _returnvalue_y))

(event `self.ReceiveBeginPlay`
  ;[1 1 1] BeginPlay
  (set `self.PlayerControllerRef` (cast `/Game/KenshilikeGame/Blueprints/Player/PlayerController_BP` (`GameplayStatics.GetPlayerController` 0) :!pure true)))

(event `self.ReceiveDrawHUD`
  (params (SizeX :type Integer) (SizeY :type Integer))
  ;[1 1 1] SelectingUnits
  (if (`self.IsDrawing`)
    (`|ExecutionSequence`
      (:`then_0`
        (`self.DrawMarquee`))
      (:`then_1`
        (set `self.UnitInSelectionArea` (`self.GetActorsInSelectionRectangle` "/Game/KenshilikeGame/Blueprints/Units/UnitMasterBP.UnitMasterBP_C" (`self.ClickLocation`) (`self.HoldingLocation`) false)))
      (:`then_2`
        ;;[1 1 1] SelectingVehicles
        (set `self.VehiclesInSelectionArea` (`self.GetActorsInSelectionRectangle` "/Game/KenshilikeGame/Blueprints/Units/Vehicles/VehicleMaster_BP.VehicleMaster_BP_C" (`self.ClickLocation`) (`self.HoldingLocation`) false))))))

(event `/Game/KenshilikeGame/Blueprints/Libraries/MarqueeSelection_BP.OnInputHold`
  (bind (_locationx _locationy) (`PlayerController.GetMousePosition` (`self.PlayerControllerRef`)))
  ;[1 1 1] OnInputHold
  (set `self.HoldingLocation` (`KismetMathLibrary.MakeVector2D` _locationx _locationy)))

(fn `ClearSelectedUnits`
  (for _array_element (`self.SelectedUnits`)
    (`/Game/KenshilikeGame/Blueprints/Units/UnitMasterBP.SetDeselectedDecal` _array_element)
    (set `/Game/KenshilikeGame/Blueprints/Units/UnitMasterBP.IsSelected?` false _array_element)
    (set `/Game/KenshilikeGame/Blueprints/Player/PlayerController_BP.IsUnitSelected?` false (`self.PlayerControllerRef`)))
  (`KismetArrayLibrary.Array_Clear` (`self.SelectedUnits`)))

(fn `ClearSelectedVehicles`
  (for _array_element (`self.Selected Vehicles`)
    (`/Game/KenshilikeGame/Blueprints/Units/Vehicles/VehicleMaster_BP.SetDeselectedDecal` _array_element)
    (set `/Game/KenshilikeGame/Blueprints/Units/Vehicles/VehicleMaster_BP.IsSelected?` false _array_element)
    (set `/Game/KenshilikeGame/Blueprints/Player/PlayerController_BP.IsUnitSelected?` false (`self.PlayerControllerRef`)))
  (`KismetArrayLibrary.Array_Clear` (`self.Selected Vehicles`)))

(fn `SetUnits`
  (bind _selectedunits (`self.SelectedUnits`))
  (for _array_element (`self.UnitInSelectionArea`)
    (if (`KismetMathLibrary.ClassIsChildOf` (`GameplayStatics.GetObjectClass` _array_element) "/Game/KenshilikeGame/Blueprints/Units/UnitMasterBP.UnitMasterBP_C")
      (bind _asunit_master_bp (cast `/Game/KenshilikeGame/Blueprints/Units/UnitMasterBP` _array_element))
      (set `self.SelectedUnit` _asunit_master_bp)
      (`|ExecutionSequence`
        (:`then_0`
          (`KismetArrayLibrary.Array_AddUnique` _selectedunits (`self.SelectedUnit`)))
        (:`then_1`
          (for _array_element_2 _selectedunits
            (`/Game/KenshilikeGame/Blueprints/Units/UnitMasterBP.SetSelectedDecal` _array_element_2)
            (set `/Game/KenshilikeGame/Blueprints/Units/UnitMasterBP.IsSelected?` true _array_element_2)))))))

(fn `SetVehicles`
  (for _array_element (`self.VehiclesInSelectionArea`)
    (if (`KismetMathLibrary.ClassIsChildOf` (`GameplayStatics.GetObjectClass` _array_element) "/Game/KenshilikeGame/Blueprints/Units/Vehicles/VehicleMaster_BP.VehicleMaster_BP_C")
      (bind _asvehicle_master_bp (cast `/Game/KenshilikeGame/Blueprints/Units/Vehicles/VehicleMaster_BP` _array_element))
      (set `self.SelectedVehicle` _asvehicle_master_bp)
      (`|ExecutionSequence`
        (:`then_0`
          (`KismetArrayLibrary.Array_AddUnique` (`self.Selected Vehicles`) (`self.SelectedVehicle`)))
        (:`then_1`
          (for _array_element_2 (`self.Selected Vehicles`)
            (`/Game/KenshilikeGame/Blueprints/Units/Vehicles/VehicleMaster_BP.SetSelectedDecal` _array_element_2)
            (set `/Game/KenshilikeGame/Blueprints/Units/Vehicles/VehicleMaster_BP.IsSelected?` false _array_element_2)))))))

(fn `UserConstructionScript`)