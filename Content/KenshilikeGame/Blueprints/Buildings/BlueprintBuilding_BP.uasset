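; Building placement preview actor that shows a ghost mesh of the selected building and toggles the player controller's building mode.
; While a gate is open, Tick snaps it to a grid at the supplied cursor position and swaps materials on overlap.
; ConstructBuilding briefly spawns the building class to read its mesh and construction work for the preview.
; SetConstructionStructure packages class, transform, mesh and construction time into a struct.
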(event `self.ReceiveTick`
  (params (DeltaSeconds :type "Float (single-precision)"))
  (bind _blueprintbuildingmesh (`self.BlueprintBuildingMesh`))
  ;[1 1 1] SetPreviewLoaction
  (`/Engine/EditorBlueprintResources/StandardMacros.Gate` true :!label _label
    (:`Exit`
      (`self.K2_SetActorLocation` self (`self.GridSnap`) false false)
      ;[1 1 1] Check if Overlapping and set material
      (if (`self.CheckOverlap`)
        (`PrimitiveComponent.SetMaterial` _blueprintbuildingmesh 0 "/Game/KenshilikeGame/Blueprints/Materials/Construction/PreviewBad_M_Inst1.PreviewBad_M_Inst1")
        (else
          (`PrimitiveComponent.SetMaterial` _blueprintbuildingmesh 0 "/Game/KenshilikeGame/Blueprints/Materials/Construction/Preview_M_Inst.Preview_M_Inst"))))))

(event `OpenGate`
  ;[1 1 1] SetPreviewLoaction
  (goto _label :!via `Open`))

(event `CloseGate`
  ;[1 1 1] SetPreviewLoaction
  (goto _label :!via `Close`))

(event `SpawnBlueprint`
  (params (BuildingClass :type "/Game/KenshilikeGame/Blueprints/Buildings/BuildingMaster_BP Class Reference") (DisplayMesh :type "StaticMesh Object Reference") (ConstructionTime :type "Float (double-precision)"))
  ;[1 1 1] SpawnBlueprint
  (if (`self.IsBlueprintON`)
    (`self.DestroyBlueprint`))
  (`self.SetBuildingDetails` ConstructionTime BuildingClass DisplayMesh)
  (bind _output_get (set `self.IsBlueprintON` true))
  (`/Game/KenshilikeGame/Blueprints/Player/PlayerController_BP.SetBuildingModeActive` (`self.PlayerControllerRef`) _output_get)
  (`StaticMeshComponent.SetStaticMesh` (`self.BlueprintBuildingMesh`) (`self.DisplayMesh`))
  (`self.OpenGate`))

(event `DestroyBlueprint`
  ;[1 1 1] DestroyBlueprint
  (`self.CloseGate`)
  (set `self.BuildingClass` null)
  (set `self.DisplayMesh` null)
  (bind _output_get (set `self.IsBlueprintON` false))
  (`/Game/KenshilikeGame/Blueprints/Player/PlayerController_BP.SetBuildingModeActive` (`self.PlayerControllerRef`) _output_get)
  (`StaticMeshComponent.SetStaticMesh` (`self.BlueprintBuildingMesh`) (`self.DisplayMesh`))
  (`self.K2_SetActorRotation` (struct)))

(event `/Game/KenshilikeGame/Blueprints/Libraries/ConstructionInterface_BP.ConstructBuilding`
  (params (BuildingMasterClass :type "/Game/KenshilikeGame/Blueprints/Buildings/BuildingMaster_BP Class Reference"))
  ;[1 1 1] ConstructBlueprint
  (bind _returnvalue (`|SpawnActorFromClass` BuildingMasterClass (`self.EmptyTransform`) "AlwaysSpawn" "OverrideRootScale" null (`self.PlayerControllerRef`) null false null))
  (`|ExecutionSequence`
    (:`then_0`
      (bind _asbuilding_master_bp (castclass `/Game/KenshilikeGame/Blueprints/Buildings/BuildingMaster_BP` BuildingMasterClass))
      (`self.DestroyBlueprint`)
      (`self.SpawnBlueprint` _asbuilding_master_bp (`/Game/KenshilikeGame/Blueprints/Buildings/BuildingMaster_BP.DisplayMesh` _returnvalue) (`/Game/KenshilikeGame/Blueprints/Buildings/BuildingMaster_BP.ConstructionWork` _returnvalue)))
    (:`then_1`
      (`self.K2_DestroyActor` _returnvalue))))

(fn `CheckOverlap`
  (returns (`isOverlaping?` :type Boolean))
  (return (>= (`KismetArrayLibrary.Array_LastIndex` (`self.GetOverlappingActors` null)) 0)))

(fn `GetCursorPosition`
  (params (CursorLocationIn :type "Vector Structure"))
  (returns (Output_Get :type "Vector Structure"))
  (bind _output_get (set `self.CursorWorldPosition` CursorLocationIn))
  (return _output_get))

(fn `GridSnap`
  (returns (SnapPosition :type "Vector Structure"))
  (bind (_cursorworldposition_x _cursorworldposition_y _cursorworldposition_z) (`KismetMathLibrary.BreakVector` (`self.CursorWorldPosition`)))
  (bind _snapvalue (`self.SnapValue`))
  (bind _snapvalue_2 (`self.SnapValue`))
  (return (`KismetMathLibrary.MakeVector` (`KismetMathLibrary.Conv_IntToDouble` (* (/ (`KismetMathLibrary.FFloor` (+ _cursorworldposition_x 50.0)) _snapvalue_2) _snapvalue_2)) (`KismetMathLibrary.Conv_IntToDouble` (* (/ (`KismetMathLibrary.FFloor` (+ _cursorworldposition_y 50.0)) _snapvalue) _snapvalue)) _cursorworldposition_z)))

(fn `SetBuildingDetails`
  (params (`Construction Time` :type "Float (double-precision)") (BuildingClass :type "/Game/KenshilikeGame/Blueprints/Buildings/BuildingMaster_BP Class Reference") (DisplayMesh :type "StaticMesh Object Reference"))
  (set `self.Construction Time` `Construction Time`)
  (set `self.BuildingClass` BuildingClass)
  (set `self.DisplayMesh` DisplayMesh))

(fn `SetConstructionStructure`
  (returns (Construction_Stuct :type "/Game/KenshilikeGame/Blueprints/Structs/Construction_Struct Structure"))
  (set `self.Construction_Struct` (make `/Game/KenshilikeGame/Blueprints/Structs/Construction_Struct` false (`self.BuildingClass`) (`self.GetTransform`) (`self.DisplayMesh`) (`self.Construction Time`)))
  (return (`self.Construction_Struct`)))

(fn `UserConstructionScript`)