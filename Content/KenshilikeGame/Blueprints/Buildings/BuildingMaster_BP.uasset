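; Master building actor that handles timed construction, unit entry, HUD info display and deletion.
; While under construction, Tick counts overlapping units as workers, advances a game-speed-scaled clock when any are present, and completes once clock × modifier × current workers reaches the required work.
; Units targeting a built, usable building trigger their arrival and move above it on overlap.
; The construction script sets the mesh and stats, while deletion destroys the actor without refunding resources.
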(event `self.ReceiveTick`
  (params (DeltaSeconds :type "Float (single-precision)"))
  ;[1 1 1] EventTick
  (set `self.DeltaTime` DeltaSeconds)
  ;;[1 1 1] Check if under construction or is it already build
  (if (and (`self.isUnderConstruction?`) (not (`self.isBuild?`)))
    ;;[1 1 1] SetWorkersAmount
    (set `self.Workers` (`KismetArrayLibrary.Array_Length` (`PrimitiveComponent.GetOverlappingActors` (`self.InteractCollision`) "/Game/KenshilikeGame/Blueprints/Units/UnitMasterBP.UnitMasterBP_C")))
    ;;[1 1 1] CheckIfThereAreWorkersPresent
    (if (> (`self.Workers`) 0)
      ;;[1 1 1] Get Game Time
      (set `self.GameClock` (`/Game/KenshilikeGame/Blueprints/Libraries/FunctionLibrary_BP.SetGameTime` (`self.DeltaTime`) (`self.GameSpeed`) (`self.GameClock`)))
      ;;[1 1 1] Calculate Time Worked
      (set `self.WorkDone` (* (`self.GameClock`) (`self.ConstructionModifier`) 60.0 (`KismetMathLibrary.Conv_IntToDouble` (`self.Workers`))))
      ;;[1 1 1] Check if Time Worked = Construction Time
      (if (>= (`self.WorkDone`) (`self.ConstructionWork`))
        ;;[1 1 1] Construction Finished
        (set `self.isBuild?` true)
        (set `self.isUnderConstruction?` false)))))

(event `GetGameSpeed`
  (params (GameSpeed :type "Float (double-precision)"))
  ;[1 1 1] GetGameSpeed
  (set `self.GameSpeed` GameSpeed))

(event `OnSpawn`
  ;[1 1 1] OnSpawn
  (set `self.isUnderConstruction?` true))

(event `self.ReceiveBeginPlay`
  (bind _gamestateref (`self.GameStateRef`))
  ;[1 1 1] BeginPlay
  (`|ExecutionSequence`
    (:`then_0`
      (`self.ReferencesCasts`))
    (:`then_1`
      ;;[1 1 1] Set Game Speed
      (add `/Game/KenshilikeGame/Blueprints/GameSetting/GameStateBase_BP.GameSpeedControl` _gamestateref (`|CreateDelegate` :!event `GetGameSpeed`))
      (bind _gamespeed (`/Game/KenshilikeGame/Blueprints/GameSetting/GameStateBase_BP.GetGameSpeed` _gamestateref))
      (set `self.GameSpeed` _gamespeed))))

(event `DisplayBuildingHUD`
  (params (Actor :type "Actor Object Reference"))
  ;[1 1 1] DisplayBuildingInfo
  (if (== Actor self)
    (`/Game/KenshilikeGame/Blueprints/Widgets/BuildingDetails_HUD.ShowBuildingInfo` (`/Game/KenshilikeGame/Blueprints/Player/PlayerController_BP.BuildingDetailsRef_HUD` (`self.PlayerControllerRef`)) self)))

(event `self.InteractCollision.OnComponentBeginOverlap`
  (params (OverlappedComponent :type "PrimitiveComponent Object Reference") (OtherActor :type "Actor Object Reference") (OtherComp :type "PrimitiveComponent Object Reference") (OtherBodyIndex :type Integer) (bFromSweep :type Boolean) (SweepResult :type "HitResult Structure (by ref)"))
  (bind (_returnvalue_x _returnvalue_y _returnvalue_z) (`KismetMathLibrary.BreakVector` (`self.K2_GetActorLocation`)))
  (bind _unitmasterref (`self.UnitMasterRef`))
  ;[1 1 1] InteractWithBuilding
  (bind _asunit_master_bp (cast `/Game/KenshilikeGame/Blueprints/Units/UnitMasterBP` OtherActor))
  (set `self.UnitMasterRef` _asunit_master_bp)
  (if (== (`/Game/KenshilikeGame/Blueprints/Units/UnitMasterBP.TargetBuilding` (`self.UnitMasterRef`)) self)
    (if (and (`self.IsBuildingUsable?`) (`self.isBuild?`))
      ;;[1 1 1] ChangeLocation
      (`/Game/KenshilikeGame/Blueprints/Units/UnitMasterBP.ArriveAtBuilding` _unitmasterref)
      (`self.K2_SetActorLocation` _unitmasterref (`KismetMathLibrary.MakeVector` _returnvalue_x _returnvalue_y (+ _returnvalue_z 500.0)) false false))))

(event `DeleteBuilding`
  (params (TargetBuilding :type "Actor Object Reference"))
  ;[1 0 0] DeleteBuilding (make it so it gives back resources!!!!)
  (if (`self.isUnderConstruction?`)
    _
    (else
      _))
  (`self.K2_DestroyActor` TargetBuilding))

(fn `SetConstructionTime`
  (params (ConstructionTimeRaw :type "Float (double-precision)"))
  (set `self.ConstructionWork` (* ConstructionTimeRaw 60.0))
  (return))

(fn `UserConstructionScript`
  ;[1 1 1] Set Details
  (set `self.BuildingStats_Struct` (make `/Game/KenshilikeGame/Blueprints/Structs/BuildingStats_Struct` (`self.BuildingName`) (`self.BuildingCurrentHealth`) (`self.BuildingMaxHealth`)))
  ;[1 1 1] SetMeshes
  (`StaticMeshComponent.SetStaticMesh` (`self.BuildingMesh`) (`self.DisplayMesh`)))