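; Player controller for an RTS-style squad game, handling camera movement, selection, orders, building placement and HUD creation.
; BeginPlay caches camera and marquee-selection HUD references, then spawns the construction managers and UI widgets.
; Left-click marquee-selects or starts construction; right-click cancels the blueprint or routes AI and vehicle moves by hit actor class, including boarding vehicles.
; Tick updates the marquee or blueprint cursor and switches details panels; debug keys spawn units and vehicles.
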(event `self.ReceiveBeginPlay`
  ;[1 1 1] BeginPlay
  (`|ExecutionSequence`
    (:`then_0`
      (`self.ReferenceCast`))
    (:`then_1`
      ;;[1 1 1] SpawnConstructionManagers
      (bind _returnvalue (`|SpawnActorFromClass` "/Game/KenshilikeGame/Blueprints/Buildings/BlueprintBuilding_BP.BlueprintBuilding_BP_C" (`self.EmptyTransform`) "AlwaysSpawn" "OverrideRootScale" null self null))
      (set `self.ContructionBlueprintRef` _returnvalue)
      (bind _returnvalue_2 (`|SpawnActorFromClass` "/Game/KenshilikeGame/Blueprints/Buildings/ConstructionMaster_BP.ConstructionMaster_BP_C" (`self.EmptyTransform`) "Undefined" "OverrideRootScale" null self null))
      (set `self.ConstructionMasterRef` _returnvalue_2))
    (:`then_2`
      (`self.SpawnWidgets`))))

(event `self.ReceiveTick`
  (params (DeltaSeconds :type "Float (single-precision)"))
  (bind _gametimerref_hud (`self.GameTimerRef_HUD`))
  (bind _gametimerref_hud_2 (`self.GameTimerRef_HUD`))
  (bind _gametimerref_hud_3 (`self.GameTimerRef_HUD`))
  (set `self.DeltaTime` DeltaSeconds)
  (`|ExecutionSequence`
    (:`then_0`
      ;[1 1 1] CallUpdateMarqueeSelection
      (if (`self.IsHoldingInput?`)
        (`self.UpdateMarqueeSelection`)
        (else
          ;[1 1 1] Check if BuildingMode is Active and we have Blueprint
          (if (and (`self.IsBuildingModeActive?`) (!= (`self.ContructionBlueprintRef`) null))
            ;[1 1 1] Get Cursor Position
            (`/Game/KenshilikeGame/Blueprints/Buildings/BlueprintBuilding_BP.GetCursorPosition` (`self.ContructionBlueprintRef`) (`/Game/KenshilikeGame/Blueprints/Libraries/FunctionLibrary_BP.SetCursorWorldPosition` self 10000.0))))))
    (:`then_1`
      (if (> (`KismetArrayLibrary.Array_Length` (`self.SelectedUnits`)) 0) :!label _label
        (`WidgetSwitcher.SetActiveWidget` (`/Game/KenshilikeGame/Blueprints/Widgets/MainGameUI_HUD.SwitcherDetails` _gametimerref_hud_3) (`/Game/KenshilikeGame/Blueprints/Widgets/MainGameUI_HUD.UnitDetails_HUD` _gametimerref_hud_3))
        (elif (`self.isItBuilding`)
          (`WidgetSwitcher.SetActiveWidget` (`/Game/KenshilikeGame/Blueprints/Widgets/MainGameUI_HUD.SwitcherDetails` _gametimerref_hud) (`/Game/KenshilikeGame/Blueprints/Widgets/MainGameUI_HUD.BuildingDetails_HUD` _gametimerref_hud))
          (else
            (`WidgetSwitcher.SetActiveWidget` (`/Game/KenshilikeGame/Blueprints/Widgets/MainGameUI_HUD.SwitcherDetails` _gametimerref_hud_2) (`/Game/KenshilikeGame/Blueprints/Widgets/MainGameUI_HUD.UnitDetails_HUD` _gametimerref_hud_2))))))))

(event `UpdateGameHUD`
  (goto _label))

(event `AddSquadMembersAtStart`
  ;[1 0 0] Add Squad Member [InProgress]
  (bind _outactors (`GameplayStatics.GetAllActorsOfClass` "/Game/KenshilikeGame/Blueprints/Units/UnitMasterBP.UnitMasterBP_C"))
  (for _array_element _outactors
    (if (`/Game/KenshilikeGame/Blueprints/Units/UnitMasterBP.IsSquadMember` _array_element)
      _))
  (`KismetSystemLibrary.PrintString` "Squad Assembled"))

(event `Key|LeftAlt`
  (params (Key :type "Key Structure"))
  ;[1 1 1] ItemLabels
  (:`Pressed`
    (set `self.ShowItemLabels` true))
  (:`Released`
    (set `self.ShowItemLabels` false)))

(event `InputAction|ToggleInventory`
  (params (Key :type "Key Structure"))
  ;[1 1 1] Open Inventory
  (:`Pressed`
    (`/Game/KenshilikeGame/Blueprints/Widgets/MainGameUI_HUD.OpenInventory` (`self.GameTimerRef_HUD`))))

(event `MoveToVehicle`
  ;[1 1 1] MouseControls
  ;;[1 1 1] SecondaryAction (Right-Click)
  ;;;[1 1 1] MoveToCommands
  (`self.ResetTargetItemIfValid`)
  (`self.UnitMoveToMacro`
    (:`On Move Finished`
      (`self.GetInVehicle`))))

(event `MoveToItem`
  ;[1 1 1] MouseControls
  ;;[1 1 1] SecondaryAction (Right-Click)
  ;;;[1 1 1] MoveToCommands
  (set `/Game/KenshilikeGame/Blueprints/Inventory/ItemMaster_BP.CanBePickedUp?` true (`self.TargetItem`))
  (`self.UnitMoveToMacro`))

(event `InputAction|SecondaryAction`
  (params (Key :type "Key Structure"))
  (bind (_hitresult _returnvalue) (`self.GetHitResultUnderCursorByChannel` "TraceTypeQuery1"))
  (bind (_bblockinghit _binitialoverlap _time _distance _location _impactpoint _normal _impactnormal _physmat _hitactor) (`GameplayStatics.BreakHitResult` _hitresult))
  ;[1 1 1] MouseControls
  ;;[1 1 1] SecondaryAction (Right-Click)
  (:`Pressed`
    (if (`self.IsBuildingModeActive?`)
      (`/Game/KenshilikeGame/Blueprints/Buildings/BlueprintBuilding_BP.DestroyBlueprint` (`self.ContructionBlueprintRef`))
      (elif (`self.IsUnitSelected?`)
        (if _returnvalue
          (set `self.TargetLocation` _location)
          (set `self.HitActor` _hitactor)
          (`|ExecutionSequence`
            (:`then_0`
              (`self.GetUnitDetails`)
              (`self.StopPreviousCommand`)
              (`self.GetMovementTarget`
                (:`MoveToVehicle`
                  (`self.MoveToVehicle`))
                (:`MoveToBuilding`
                  (`self.MoveToBuilding`))
                (:`MoveToResource`
                  (`self.MoveToResource`))
                (:`MoveToItem`
                  (`self.MoveToItem`))
                (:`MoveToLocation`
                  (`self.MoveTo`))))
            (:`then_1`
              (`self.VehicleMovement`))))))))

(event `Key|V`
  (params (Key :type "Key Structure"))
  (bind (_relativecursorlocationingame_x _relativecursorlocationingame_y) (`KismetMathLibrary.BreakVector` (`/Game/KenshilikeGame/Blueprints/Libraries/FunctionLibrary_BP.SetCursorWorldPosition` self 10000.0)))
  ;[1 1 1] DEBUG only
  ;;[1 1 1] SpawnUnitDEBUG!!!
  (:`Pressed`
    (`|SpawnActorFromClass` "/Game/KenshilikeGame/Blueprints/Units/UnitMasterBP.UnitMasterBP_C" (`KismetMathLibrary.MakeTransform` (`KismetMathLibrary.MakeVector` _relativecursorlocationingame_x _relativecursorlocationingame_y 200.0)) "Undefined" "OverrideRootScale" null false (struct) null)))

(event `Key|LeftShift`
  (params (Key :type "Key Structure"))
  ;[1 1 1] CameraMovement
  ;;[1 1 1] ShiftOnOff
  (:`Pressed`
    (set `self.IsShiftPressed?` true))
  (:`Released`
    (set `self.IsShiftPressed?` false)))

(event `InputAction|ZoomReset`
  (params (Key :type "Key Structure"))
  ;[1 1 1] CameraMovement
  ;;[1 1 1] Zoom
  ;;;[1 1 1] ZoomReset
  (:`Pressed`
    (set `SpringArmComponent.TargetArmLength` 1500.0 (`/Game/KenshilikeGame/Blueprints/Player/CameraPawn_BP.SpringArm` (`self.CameraPawnRef`)))))

(event `MoveToBuilding`
  ;[1 1 1] MouseControls
  ;;[1 1 1] SecondaryAction (Right-Click)
  ;;;[1 1 1] MoveToCommands
  (`self.ResetTargetItemIfValid`)
  (`/Game/KenshilikeGame/Blueprints/Units/UnitMasterBP.GetTargetBuilding` (`self.SelectedUnit`) (`self.TargetBuilding`))
  (`self.UnitMoveToMacro`))

(event `InputAction|Pan`
  (params (Key :type "Key Structure"))
  (bind _stopcammovementwhenpanningzooming_ (`self.StopCamMovementWhenPanningZooming?`))
  ;[1 1 1] CameraMovement
  ;;[1 1 1] StopCamMove
  (:`Pressed`
    (if _stopcammovementwhenpanningzooming_
      (set `self.StopCamMove` true)))
  (:`Released`
    (if _stopcammovementwhenpanningzooming_
      (set `self.StopCamMove` false))))

(event `MoveToResource`
  ;[1 1 1] MouseControls
  ;;[1 1 1] SecondaryAction (Right-Click)
  ;;;[1 1 1] MoveToCommands
  (`self.ResetTargetItemIfValid`))

(event `RemoveLocationDecals`
  (bind _previouslocationdecal (`self.PreviousLocationDecal`))
  ;[1 1 1] MouseControls
  ;;[1 1 1] SecondaryAction (Right-Click)
  (`/Engine/EditorBlueprintResources/StandardMacros.IsValid` _previouslocationdecal
    (:`Is Valid`
      (`ActorComponent.K2_DestroyComponent` _previouslocationdecal))))

(event `InputAction|ZoomIn`
  (params (Key :type "Key Structure"))
  (bind _springarm (`/Game/KenshilikeGame/Blueprints/Player/CameraPawn_BP.SpringArm` (`self.CameraPawnRef`)))
  ;[1 1 1] CameraMovement
  ;;[1 1 1] Zoom
  ;;;[1 1 1] ZoomInOut
  (:`Pressed`
    (set `SpringArmComponent.TargetArmLength` (`KismetMathLibrary.FClamp` (- (`SpringArmComponent.TargetArmLength` _springarm) (`self.ZoomSensitivity`)) (`self.ZoomMinLimit`) (`self.ZoomMaxLimit`)) _springarm)))

(event `MoveTo`
  ;[1 1 1] MouseControls
  ;;[1 1 1] SecondaryAction (Right-Click)
  ;;;[1 1 1] MoveToCommands
  (`self.ResetTargetItemIfValid`)
  (`self.UnitMoveToMacro`
    (:`On Move Finished`
      (`self.RemoveLocationDecals`))))

(event `Key|B`
  (params (Key :type "Key Structure"))
  (bind (_relativecursorlocationingame_x _relativecursorlocationingame_y) (`KismetMathLibrary.BreakVector` (`/Game/KenshilikeGame/Blueprints/Libraries/FunctionLibrary_BP.SetCursorWorldPosition` self 10000.0)))
  ;[1 1 1] DEBUG only
  ;;[1 1 1] SpawnVehicleDEBUG!!!
  (:`Pressed`
    (`|SpawnActorFromClass` "/Game/KenshilikeGame/Blueprints/Units/Vehicles/VehicleMaster_BP.VehicleMaster_BP_C" (`KismetMathLibrary.MakeTransform` (`KismetMathLibrary.MakeVector` _relativecursorlocationingame_x _relativecursorlocationingame_y 200.0)) "Undefined" "OverrideRootScale" null "NewEnumerator0" null)))

(event `InputAxis|MoveForward`
  (params (AxisValue :type "Float (single-precision)"))
  ;[1 1 1] CameraMovement
  ;;[1 1 1] MoveXY
  (if (not (`self.StopCamMove`))
    (`self.MoveXY` AxisValue (stale `InputAxis|MoveRight` AxisValue) :!label _label_2)))

(event `InputAction|ZoomOut`
  (params (Key :type "Key Structure"))
  (bind _springarm (`/Game/KenshilikeGame/Blueprints/Player/CameraPawn_BP.SpringArm` (`self.CameraPawnRef`)))
  ;[1 1 1] CameraMovement
  ;;[1 1 1] Zoom
  ;;;[1 1 1] ZoomInOut
  (:`Pressed`
    (set `SpringArmComponent.TargetArmLength` (`KismetMathLibrary.FClamp` (+ (`self.ZoomSensitivity`) (`SpringArmComponent.TargetArmLength` _springarm)) (`self.ZoomMinLimit`) (`self.ZoomMaxLimit`)) _springarm)))

(event `InputAxis|MoveRight`
  (params (AxisValue :type "Float (single-precision)"))
  ;[1 1 1] CameraMovement
  ;;[1 1 1] MoveXY
  (if (not (`self.StopCamMove`))
    (goto _label_2 :!via `RightMovement`)))

(event `StartMarqueeSelect`
  ;[1 1 1] MouseControls
  ;;[1 1 1] PrimaryAction (Left-Click)
  ;;;[1 1 1] MarqueeSelection
  ;;;;[1 1 1] On Left Click
  (message `/Game/KenshilikeGame/Blueprints/Libraries/MarqueeSelection_BP.OnInputStart` (`self.MarquessSlectionRef`))
  (set `self.HoldingTime` 0.0)
  (set `self.IsHoldingInput?` true))

(event `InputAction|PrimaryAction`
  (params (Key :type "Key Structure"))
  (bind (_returnvalue _hitactor) (`self.isItBuilding`))
  (bind _marquessslectionref (`self.MarquessSlectionRef`))
  ;[1 1 1] MouseControls
  ;;[1 1 1] PrimaryAction (Left-Click)
  (:`Pressed`
    (if (`self.IsBuildingModeActive?`)
      (`self.BeginConstruction`)
      (else
        (`self.StartMarqueeSelect`)
        (if _returnvalue
          (`self.GetBuildingHud` _hitactor)))))
  (:`Released`
    (if (not (`self.IsBuildingModeActive?`))
      (message `/Game/KenshilikeGame/Blueprints/Libraries/MarqueeSelection_BP.OnInputRelease` _marquessslectionref (`self.HoldingTime`))
      (set `self.IsHoldingInput?` false)
      (`self.GetUnitHud` (`/Game/KenshilikeGame/Blueprints/HUD/MarquessSlection_BP.SelectedUnits` _marquessslectionref)))))

(event `UpdateMarqueeSelection`
  ;[1 1 1] MouseControls
  ;;[1 1 1] PrimaryAction (Left-Click)
  ;;;[1 1 1] MarqueeSelection
  ;;;;[1 1 1] Update Mouse Location
  (if (`self.IsHoldingInput?`)
    (set `self.HoldingTime` (+ (`self.HoldingTime`) (`self.DeltaTime`)))
    (message `/Game/KenshilikeGame/Blueprints/Libraries/MarqueeSelection_BP.OnInputHold` (`self.MarquessSlectionRef`))))

(event `InputAction|Pan`
  (params (Key :type "Key Structure"))
  (bind (_returnvalue_roll _returnvalue_pitch _returnvalue_yaw) (`KismetMathLibrary.BreakRotator` (`self.K2_GetActorRotation` (`self.CameraPawnRef`))))
  ;[1 1 1] CameraMovement
  ;;[1 1 1] Pan
  ;;;[1 1 1] Pan
  (:`Pressed`
    (goto _label_3 :!via `Open`))
  (:`Released`
    (goto _label_3 :!via `Close`)))

(event `InputAxisKey|MouseX`
  (params (AxisValue :type "Float (single-precision)"))
  (bind (_returnvalue_roll _returnvalue_pitch _returnvalue_yaw) (`KismetMathLibrary.BreakRotator` (`self.K2_GetActorRotation` (`self.CameraPawnRef`))))
  ;[1 1 1] CameraMovement
  ;;[1 1 1] Pan
  ;;;[1 1 1] Pan
  (`/Engine/EditorBlueprintResources/StandardMacros.Gate` true :!label _label_3
    (:`Exit`
      (`self.K2_SetActorRotation` (`self.CameraPawnRef`) (`KismetMathLibrary.MakeRotator` _returnvalue_roll _returnvalue_pitch (+ (* AxisValue (`self.PanSensitivity`)) _returnvalue_yaw)) false))))

(event `InputAction|RotateBlueprintLeft`
  (params (Key :type "Key Structure"))
  (bind _contructionblueprintref (`self.ContructionBlueprintRef`))
  (bind (_returnvalue_roll _returnvalue_pitch _returnvalue_yaw) (`KismetMathLibrary.BreakRotator` (`self.K2_GetActorRotation` _contructionblueprintref)))
  ;[1 0.5052 0.5052] RotateBlueprintRightLeft (make it so holding a key is turning blueprint constantly!)
  (:`Pressed`
    ;;[1 1 1] Check if BuildingMode is Active and we have Blueprint
    (if (and (`self.IsBuildingModeActive?`) (!= _contructionblueprintref null))
      (`self.K2_SetActorRotation` _contructionblueprintref (`KismetMathLibrary.MakeRotator` _returnvalue_roll _returnvalue_pitch (+ _returnvalue_yaw (`self.ConstructionBlueprintRotationRate`))) false))))

(event `InputAction|Pan`
  (params (Key :type "Key Structure"))
  (bind (_returnvalue_roll _returnvalue_pitch _returnvalue_yaw) (`KismetMathLibrary.BreakRotator` (`self.K2_GetActorRotation` (`self.CameraPawnRef`))))
  ;[1 1 1] CameraMovement
  ;;[1 1 1] Pan
  ;;;[1 1 1] Pan
  (:`Pressed`
    (goto _label_4 :!via `Open`))
  (:`Released`
    (goto _label_4 :!via `Close`)))

(event `InputAxisKey|MouseY`
  (params (AxisValue :type "Float (single-precision)"))
  (bind (_returnvalue_roll _returnvalue_pitch _returnvalue_yaw) (`KismetMathLibrary.BreakRotator` (`self.K2_GetActorRotation` (`self.CameraPawnRef`))))
  ;[1 1 1] CameraMovement
  ;;[1 1 1] Pan
  ;;;[1 1 1] Pan
  (`/Engine/EditorBlueprintResources/StandardMacros.Gate` true :!label _label_4
    (:`Exit`
      (`self.K2_SetActorRotation` (`self.CameraPawnRef`) (`KismetMathLibrary.MakeRotator` _returnvalue_roll (`KismetMathLibrary.FClamp` (+ (* AxisValue (`self.PanSensitivity`)) _returnvalue_pitch) -20.0 60.0) _returnvalue_yaw) false))))

(event `InputAction|RotateBlueprintRight`
  (params (Key :type "Key Structure"))
  (bind _contructionblueprintref (`self.ContructionBlueprintRef`))
  (bind (_returnvalue_roll _returnvalue_pitch _returnvalue_yaw) (`KismetMathLibrary.BreakRotator` (`self.K2_GetActorRotation` _contructionblueprintref)))
  ;[1 0.5052 0.5052] RotateBlueprintRightLeft (make it so holding a key is turning blueprint constantly!)
  (:`Pressed`
    ;;[1 1 1] Check if BuildingMode is Active and we have Blueprint
    (if (and (`self.IsBuildingModeActive?`) (!= _contructionblueprintref null))
      (`self.K2_SetActorRotation` _contructionblueprintref (`KismetMathLibrary.MakeRotator` _returnvalue_roll _returnvalue_pitch (- _returnvalue_yaw (`self.ConstructionBlueprintRotationRate`))) false))))

(event `InputAction|PanReset`
  (params (Key :type "Key Structure"))
  (bind _camerapawnref (`self.CameraPawnRef`))
  (bind _returnvalue_roll (`KismetMathLibrary.BreakRotator` (`self.K2_GetActorRotation` _camerapawnref)))
  ;[1 1 1] CameraMovement
  ;;[1 1 1] Pan
  ;;;[1 1 1] PanReset
  (:`Pressed`
    (`self.K2_SetActorRotation` _camerapawnref (`KismetMathLibrary.MakeRotator` _returnvalue_roll) false)))

(fn `GetBuildingHud`
  (params (Actor :type "Actor Object Reference"))
  (if (!= (`.HitActor` (`GameplayStatics.BreakHitResult` (`self.GetHitResultUnderCursorForObjects` (`self.SelectableObjectsEnum`)))) null)
    (`/Game/KenshilikeGame/Blueprints/Buildings/BuildingMaster_BP.DisplayBuildingHUD` (cast `/Game/KenshilikeGame/Blueprints/Buildings/BuildingMaster_BP` Actor :!pure true) Actor)))

(fn `GetUnitHud`
  (params (SelectedUnits :type "Array of /Game/KenshilikeGame/Blueprints/Units/UnitMasterBP Object Reference"))
  (if (!= (`.HitActor` (`GameplayStatics.BreakHitResult` (`self.GetHitResultUnderCursorForObjects` (`self.SelectableObjectsEnum`)))) null)
    (`self.DisplayUnitHud` (`|GetArrayItem` SelectedUnits (`KismetMathLibrary.RandomIntegerInRange` 0 (- (`KismetArrayLibrary.Array_Length` SelectedUnits) 1))))))

(fn `isItBuilding`
  (returns (ReturnValue :type Boolean) (HitActor :type "Actor Object Reference"))
  (bind (_bblockinghit _binitialoverlap _time _distance _location _impactpoint _normal _impactnormal _physmat _hitactor) (`GameplayStatics.BreakHitResult` (`self.GetHitResultUnderCursorForObjects` (`self.SelectableObjectsEnum`))))
  (return (`KismetMathLibrary.ClassIsChildOf` (`GameplayStatics.GetObjectClass` _hitactor) "/Game/KenshilikeGame/Blueprints/Buildings/BuildingMaster_BP.BuildingMaster_BP_C") _hitactor))

(fn `ResetTargetItemIfValid`
  (bind _targetitem (`self.TargetItem`)
    (:`then`
      (set `/Game/KenshilikeGame/Blueprints/Inventory/ItemMaster_BP.CanBePickedUp?` false _targetitem))
    (:`else`)))

(fn `Set Selected Units`
  (params (SelectedUnits :type "Array of /Game/KenshilikeGame/Blueprints/Units/UnitMasterBP Object Reference") (SelectedVehicles :type "Array of /Game/KenshilikeGame/Blueprints/Units/Vehicles/VehicleMaster_BP Object Reference"))
  (set `self.SelectedUnits` SelectedUnits)
  (set `self.SelectedVehicles` SelectedVehicles)
  (if (or (>= (`KismetArrayLibrary.Array_LastIndex` (`self.SelectedUnits`)) 0) (>= (`KismetArrayLibrary.Array_LastIndex` (`self.SelectedVehicles`)) 0) false)
    (set `self.IsUnitSelected?` true)))

(fn `SetBuildingModeActive`
  (params (`IsActive?` :type Boolean))
  (set `self.IsBuildingModeActive?` `IsActive?`)
  (return))

(fn `StopPreviousCommand`
  (bind _previouslocationdecal (`self.PreviousLocationDecal`))
  ;[1 1 1] RemoveMoveDecal
  (`/Engine/EditorBlueprintResources/StandardMacros.IsValid` _previouslocationdecal
    (:`Is Valid`
      (`ActorComponent.K2_DestroyComponent` _previouslocationdecal))
    (:`Is Not Valid`
      _))
  (`/Game/KenshilikeGame/Blueprints/Units/UnitMasterBP.TargetBuilding` (`self.SelectedUnit`)
    (:`then`
      (set `/Game/KenshilikeGame/Blueprints/Units/UnitMasterBP.TargetBuilding` null (`self.SelectedUnit`)))
    (:`else`
      _))
  ;[1 0.8131 0] Wywołuje lagowanie postaci
  (`self.StopMovement` (`self.UnitAI`))
  (return))

(fn `UserConstructionScript`)