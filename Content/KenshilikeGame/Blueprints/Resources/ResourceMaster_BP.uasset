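; ResourceMaster_BP is a resource node, apparently the master for ore, scrap and wood resources.
; Its construction script randomly rescales the mesh relative to its current scale and independently rolls an amount, weighted by resource type and floored.
; At BeginPlay it caches game state and player controller references, then binds to game speed changes and stores the current speed.
; Calendar and clock functions are empty stubs returning false.
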(event `self.ReceiveBeginPlay`
  (bind _gamestateref (`self.GameStateRef`))
  (`|ExecutionSequence`
    (:`then_0`
      ;[1 1 1] Reference Casts
      (`self.ReferenceCasts`))
    (:`then_1`
      ;[1 1 1] Set Game Speed
      (add `/Game/KenshilikeGame/Blueprints/GameSetting/GameStateBase_BP.GameSpeedControl` _gamestateref (`|CreateDelegate` :!event `GetGameSpeed`))
      (bind _gamespeed (`/Game/KenshilikeGame/Blueprints/GameSetting/GameStateBase_BP.GetGameSpeed` _gamestateref))
      (set `self.GameSpeed` _gamespeed))))

(event `GetGameSpeed`
  (params (GameSpeed :type "Float (double-precision)"))
  ;[1 1 1] Set Game Speed
  (set `self.GameSpeed` GameSpeed))

(fn `RescaleMesh`
  (returns (ReturnValue :type "Float (double-precision)") (ReturnValue2 :type "Float (double-precision)") (ReturnValue3 :type "Float (double-precision)"))
  (bind _meshscale (`self.MeshScale`))
  (bind (_returnvalue_x _returnvalue_y _returnvalue_z) (`KismetMathLibrary.BreakVector` (`SceneComponent.K2_GetComponentScale` (`self.ResourceMesh`))))
  (return (* _returnvalue_x _meshscale) (* _returnvalue_y _meshscale) (* _returnvalue_z _meshscale)))

(fn `SetGameCalendar`
  (params (GameDate :type "Array of Integer (by ref)"))
  (returns (Success :type Boolean))
  (return false))

(fn `SetGameClock`
  (params (GameTime :type "Array of Integer (by ref)"))
  (returns (Success :type Boolean))
  (return false))

(fn `SetResourceAmount`
  (returns (Output_Get :type "Float (double-precision)"))
  (bind _output_get (set `self.ResourceAmount` (`KismetMathLibrary.Conv_IntToDouble` (`KismetMathLibrary.FFloor` (* (`self.ResourceAmount`) (`self.ResourceMultiplier`))))))
  (return _output_get))

(fn `UserConstructionScript`
  (bind (_returnvalue _returnvalue2 _returnvalue3) (`self.RescaleMesh`))
  (set `self.MeshScale` (`KismetMathLibrary.RandomFloatInRange` 0.5 5.0))
  (`SceneComponent.SetWorldScale3D` (`self.ResourceMesh`) (`KismetMathLibrary.MakeVector` _returnvalue _returnvalue2 _returnvalue3))
  ;[1 1 1] Set Resource Amount to Resource Type
  (`self.CheckResourceType`
    (:`Ore`
      (set `self.ResourceMultiplier` 1.0))
    (:`Scrap`
      (set `self.ResourceMultiplier` 0.8))
    (:`Wood`
      (set `self.ResourceMultiplier` 1.5)))
  ;[1 1 1] Set Random Resource Amount
  (set `self.ResourceAmount` (`KismetMathLibrary.RandomFloatInRange` 50.0 200.0))
  (`self.SetResourceAmount`))